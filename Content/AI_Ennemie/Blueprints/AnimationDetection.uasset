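; Behavior Tree task that plays the enemy's reaction when it detects the player.
; It plays a detection sound on every execution, but runs the montage only when MannequinMasterAi's 20SecTimer equals 20, setting flags that start that pawn's cooldown.
; Movement is disabled during the montage to prevent sliding, then restored to NavWalking on completion.
; While the task runs, its tick turns the enemy toward the player.
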(event `self.ReceiveExecuteAI`
  (params (OwnerController :type "AIController Object Reference") (ControlledPawn :type "Pawn Object Reference"))
  ;[1 1 1] Activation du timer et de l'animation de détection
  (bind _asmannequin_master_ai (cast `/Game/AI_Ennemie/Blueprints/MannequinMasterAi` ControlledPawn))
  (`GameplayStatics.PlaySound2D` "/Game/Sound/Attaque/Detection.Detection" 1.0 1.0 0.0 null null)
  (if (== (`/Game/AI_Ennemie/Blueprints/MannequinMasterAi.20SecTimer` _asmannequin_master_ai) 20.0)
    ;;[1 1 1] Si c'est vrai , on active ces booléan pour commencer le timer qui est situé dans le BP du AI
    (set `/Game/AI_Ennemie/Blueprints/MannequinMasterAi.StartDetectionAnimCoolDownTimer` true _asmannequin_master_ai)
    (set `/Game/AI_Ennemie/Blueprints/MannequinMasterAi.DetectedPlayer` true _asmannequin_master_ai)
    (bind _charactermovement (`Character.CharacterMovement` _asmannequin_master_ai))
    (`CharacterMovementComponent.DisableMovement` _charactermovement) ; On désactive le mouvement pour que le AI ne glisse pas lors de l'animation
    (`|PlayMontage` (`Character.Mesh` _asmannequin_master_ai) (`self.AnimDetection`)
      (:`OnCompleted`
        (`CharacterMovementComponent.SetMovementMode` _charactermovement "MOVE_NavWalking" 0)
        (`self.FinishExecute` true)))
    (else
      (`self.FinishExecute` true))))

(event `self.ReceiveTickAI`
  (params (OwnerController :type "AIController Object Reference") (ControlledPawn :type "Pawn Object Reference") (DeltaSeconds :type "Float (single-precision)"))
  ;[1 1 1] Rotation de l'ennemie vers le joueur lorsqu'il détecte le joueur et se fixe vers le joueur pendant l'animation mais si celle-ci bouge
  (`Actor.K2_SetActorRotation` ControlledPawn (`KismetMathLibrary.FindLookAtRotation` (`Actor.K2_GetActorLocation` ControlledPawn) (`Actor.K2_GetActorLocation` (`GameplayStatics.GetPlayerCharacter` 0))) false))