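; Blueprint interface that declares the interaction messages shared between gameplay actors, with no logic of its own.
; It covers generic object interaction, lamp pickup, an on-screen interaction notification with an in/out flag, and door interaction.
; It also declares health and battery value calculations, a combined stat calculation with a memory flag, and a timed gate destruction call.
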(fn `BatterieCalcul`
  (params (ValeurPickUp :type "Float (double-precision)"))
  (return))

(fn `CalculStat`
  (params (`IsMemoire?` :type Boolean) (ValeurBattery :type "Float (double-precision)") (`ValeurSanté` :type "Float (double-precision)")))

(fn `DestructionGate`
  (params (Time :type "Float (double-precision)")))

(fn `InteractionObject`
  (return))

(fn `NotificationEcranInteraction`
  (params (`IsOut?` :type Boolean))
  (return))

(fn `PickUp_Lampe`
  (return))

(fn `Porte`
  (return))

(fn `SanteCalcul`
  (params (Valeur :type "Float (double-precision)"))
  (return))