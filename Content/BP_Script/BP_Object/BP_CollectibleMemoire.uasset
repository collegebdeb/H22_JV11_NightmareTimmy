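; Collectible memory pickup that restores the first-person character's mental health and increments their memory count.
; Tick spins the actor and plays a timeline that lerps the CollectibleSante component's height between two limits.
; Hitbox overlap enables interaction unless the character's MaxSante flag is set, and leaving disables it.
; InteractionObject, if enabled and mental health is below its limit, destroys the actor, sends the health value and increments the count.
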(event `self.ReceiveTick`
  (params (DeltaSeconds :type "Float (single-precision)"))
  (`|ExecutionSequence`
    (:`then_0`
      ;[1 1 1] Rotation de la batterie selon le temps
      (`self.K2_AddActorLocalRotation` (* (`KismetMathLibrary.MakeRotator` 0.0 0.0 (`self.RotationCollectible`)) DeltaSeconds)))
    (:`then_1`
      ;[1 1 1] Permet de créer une animation en translation interpolé selon l'alpha d'un timeline
      (bind (_direction _alpha) (`Timeline|Timeline_0`)
        (:`Update`
          (`SceneComponent.K2_SetRelativeLocation` (`self.CollectibleSante`) (`KismetMathLibrary.VLerp` (`KismetMathLibrary.MakeVector` 0.0 0.0 (`self.ValeurTranslationMax`)) (`KismetMathLibrary.MakeVector` 0.0 0.0 (`self.ValeurTranslationMin`)) _alpha) false false))))))

(event `self.Hitbox.OnComponentBeginOverlap`
  (params (OverlappedComponent :type "PrimitiveComponent Object Reference") (OtherActor :type "Actor Object Reference") (OtherComp :type "PrimitiveComponent Object Reference") (OtherBodyIndex :type Integer) (bFromSweep :type Boolean) (SweepResult :type "HitResult Structure (by ref)"))
  ;[1 1 1] Si la batterie est plus petite et que le personnage est proche de l'objet, permet d'intéragir avec celui-ci
  (bind _asbp_first_person_character (cast `/Game/FirstPersonBP/Blueprints/BP_FirstPersonCustom/BP_FirstPersonCharacter` OtherActor))
  (set `self.BP_FirstPerson` _asbp_first_person_character)
  (if (not (`/Game/FirstPersonBP/Blueprints/BP_FirstPersonCustom/BP_FirstPersonCharacter.MaxSante?` (`self.BP_FirstPerson`)))
    (set `self.CanInteract?` true)))

(event `self.Hitbox.OnComponentEndOverlap`
  (params (OverlappedComponent :type "PrimitiveComponent Object Reference") (OtherActor :type "Actor Object Reference") (OtherComp :type "PrimitiveComponent Object Reference") (OtherBodyIndex :type Integer))
  ;[1 1 1] Lorsque le personnage est plu dans la zone, ne peut plu intéragir avec l'objet
  (cast `/Game/FirstPersonBP/Blueprints/BP_FirstPersonCustom/BP_FirstPersonCharacter` OtherActor)
  (set `self.CanInteract?` false))

(event `/Game/BP_Script/BP_Interface/BP_Interface_Interact.InteractionObject`
  (bind _bp_firstperson (`self.BP_FirstPerson`))
  ;[1 1 1] Calcul de la valeur de l'obtention lors du PickUp de l'objet au sol
  (if (and (> (`/Game/FirstPersonBP/Blueprints/BP_FirstPersonCustom/BP_FirstPersonCharacter.LimitSanteMentale` _bp_firstperson) (`/Game/FirstPersonBP/Blueprints/BP_FirstPersonCustom/BP_FirstPersonCharacter.SanteMentale` _bp_firstperson)) (`self.CanInteract?`))
    (`self.K2_DestroyActor`)
    (message `/Game/BP_Script/BP_Interface/BP_Interface_Interact.SanteCalcul` _bp_firstperson (`self.ValeurSante`))
    (`/Engine/EditorBlueprintResources/StandardMacros.IncrementInt` (`/Game/FirstPersonBP/Blueprints/BP_FirstPersonCustom/BP_FirstPersonCharacter.MemoryCount` _bp_firstperson))))

(fn `UserConstructionScript`)