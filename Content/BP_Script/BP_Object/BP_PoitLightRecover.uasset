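; A placeable spot light that switches the first-person character's sanity state, apparently acting as a recovery zone.
; A capsule hitbox calls SanityMessage on the player when overlap begins and PerteSanityMessage (French for loss) when it ends.
; The construction script applies variables to the light's transform, intensity, cone and radius, and to the hitbox's size and position, so each instance is tunable.
; Despite the asset's name, the light is a spot light.
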(event `self.Hitbox.OnComponentBeginOverlap`
  (params (OverlappedComponent :type "PrimitiveComponent Object Reference") (OtherActor :type "Actor Object Reference") (OtherComp :type "PrimitiveComponent Object Reference") (OtherBodyIndex :type Integer) (bFromSweep :type Boolean) (SweepResult :type "HitResult Structure (by ref)"))
  (bind _asbp_first_person_character (cast `/Game/FirstPersonBP/Blueprints/BP_FirstPersonCustom/BP_FirstPersonCharacter` OtherActor))
  (message `/Game/BP_Script/BP_Interface/BP_Interface_PerteSanity.Sanity` _asbp_first_person_character))

(event `self.Hitbox.OnComponentEndOverlap`
  (params (OverlappedComponent :type "PrimitiveComponent Object Reference") (OtherActor :type "Actor Object Reference") (OtherComp :type "PrimitiveComponent Object Reference") (OtherBodyIndex :type Integer))
  (bind _asbp_first_person_character (cast `/Game/FirstPersonBP/Blueprints/BP_FirstPersonCustom/BP_FirstPersonCharacter` OtherActor))
  (message `/Game/BP_Script/BP_Interface/BP_Interface_PerteSanity.PerteSanity` _asbp_first_person_character))

(fn `UserConstructionScript`
  (bind _hitbox (`self.Hitbox`))
  (bind _spotlight (`self.SpotLight`))
  (`|ExecutionSequence`
    (:`then_0`
      (`SceneComponent.K2_SetRelativeLocationAndRotation` (`self.SpotLight`) (`self.LocationLight`) (`self.RotatorLight`) false false)
      (`LightComponent.SetIntensity` _spotlight (`self.Intensity`))
      (`SpotLightComponent.SetOuterConeAngle` _spotlight (`self.OuterConeAngle`))
      (`LocalLightComponent.SetAttenuationRadius` _spotlight (`self.AttenuationRadius`)))
    (:`then_1`
      (`CapsuleComponent.SetCapsuleSize` _hitbox (`self.InRadius`) (`self.HalfHeight`) true)
      (`SceneComponent.K2_SetRelativeLocation` _hitbox (`self.LocationHitbox`) false false))))