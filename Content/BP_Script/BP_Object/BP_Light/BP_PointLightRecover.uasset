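; BP_PointLightRecover is a point light with a sphere hitbox, apparently marking a zone that affects the player's sanity.
; When a BP_FirstPersonCharacter enters the sphere it calls SanityMessage on that character, and on exit it calls PerteSanityMessage.
; The construction script applies exposed variables to the light's intensity, attenuation and source radius, and to the hitbox's position and radius.
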(event `self.Hitbox.OnComponentBeginOverlap`
  (params (OverlappedComponent :type "PrimitiveComponent Object Reference") (OtherActor :type "Actor Object Reference") (OtherComp :type "PrimitiveComponent Object Reference") (OtherBodyIndex :type Integer) (bFromSweep :type Boolean) (SweepResult :type "HitResult Structure (by ref)"))
  (bind _asbp_first_person_character (cast `/Game/FirstPersonBP/Blueprints/BP_FirstPersonCustom/BP_FirstPersonCharacter` OtherActor))
  (message `/Game/BP_Script/BP_Interface/BP_Interface_PerteSanity.Sanity` _asbp_first_person_character))

(event `self.Hitbox.OnComponentEndOverlap`
  (params (OverlappedComponent :type "PrimitiveComponent Object Reference") (OtherActor :type "Actor Object Reference") (OtherComp :type "PrimitiveComponent Object Reference") (OtherBodyIndex :type Integer))
  (bind _asbp_first_person_character (cast `/Game/FirstPersonBP/Blueprints/BP_FirstPersonCustom/BP_FirstPersonCharacter` OtherActor))
  (message `/Game/BP_Script/BP_Interface/BP_Interface_PerteSanity.PerteSanity` _asbp_first_person_character))

(fn `UserConstructionScript`
  (bind _pointlight (`self.PointLight`))
  (`|ExecutionSequence`
    (:`then_0`
      (`LightComponent.SetIntensity` _pointlight (`self.Intensity`))
      (`LocalLightComponent.SetAttenuationRadius` _pointlight (`self.AttenuationRadius`))
      (`PointLightComponent.SetSourceRadius` _pointlight (`self.SourceRadius`)))
    (:`then_1`
      (`SceneComponent.K2_SetRelativeLocation` (`self.Hitbox`) (`self.LocationHitbox`) false false)
      (`SphereComponent.SetSphereRadius` (`self.Hitbox`) (`self.SphereRadius`) true))))