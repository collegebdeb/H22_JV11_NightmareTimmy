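; BP_AuraEnnemySanity is an enemy aura that drains the first-person character's mental health (SanteMentale) while the player stays inside it.
; Overlapping LightCollision caches the character and starts a looping one-second timer on DamageOverTime, which ending the overlap clears.
; Each tick subtracts DommageOverTime from SanteMentale and prints the new value, with no clamping in this Blueprint.
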(event `self.LightCollision.OnComponentBeginOverlap`
  (params (OverlappedComponent :type "PrimitiveComponent Object Reference") (OtherActor :type "Actor Object Reference") (OtherComp :type "PrimitiveComponent Object Reference") (OtherBodyIndex :type Integer) (bFromSweep :type Boolean) (SweepResult :type "HitResult Structure (by ref)"))
  ;[1 1 1] Calculer si le joueur est dans la zone d'influence
  (bind _asbp_first_person_character (cast `/Game/FirstPersonBP/Blueprints/BP_FirstPersonCustom/BP_FirstPersonCharacter` OtherActor))
  (set `self.BP_FirstPerson` _asbp_first_person_character)
  (`self.DommagePerteTime`))

(event `self.LightCollision.OnComponentEndOverlap`
  (params (OverlappedComponent :type "PrimitiveComponent Object Reference") (OtherActor :type "Actor Object Reference") (OtherComp :type "PrimitiveComponent Object Reference") (OtherBodyIndex :type Integer))
  ;[1 1 1] Calculer si le joueur est dans la zone d'influence
  (cast `/Game/FirstPersonBP/Blueprints/BP_FirstPersonCustom/BP_FirstPersonCharacter` OtherActor)
  (`self.Arrêt`))

(event `DommagePerteTime`
  ;[1 1 1] Calculer si le joueur est dans la zone d'influence
  (bind _returnvalue (`KismetSystemLibrary.K2_SetTimer` null "DamageOverTime" 1.0 true)))

(event `Arrêt`
  ;[1 1 1] Calculer si le joueur est dans la zone d'influence
  (`KismetSystemLibrary.K2_ClearAndInvalidateTimerHandle` (stale `DommagePerteTime` _returnvalue)))

(fn `DamageOverTime`
  (bind _bp_firstperson (`self.BP_FirstPerson`))
  (bind _output_get (set `/Game/FirstPersonBP/Blueprints/BP_FirstPersonCustom/BP_FirstPersonCharacter.SanteMentale` (- (`/Game/FirstPersonBP/Blueprints/BP_FirstPersonCustom/BP_FirstPersonCharacter.SanteMentale` _bp_firstperson) (`self.DommageOverTime`)) _bp_firstperson))
  (`KismetSystemLibrary.PrintString` (`KismetStringLibrary.Conv_DoubleToString` _output_get)))

(fn `UserConstructionScript`)