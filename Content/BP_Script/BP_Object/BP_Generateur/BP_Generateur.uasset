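; Generator interactable that raises a separately placed door (Cube) when the first-person player activates it.
; A hitbox overlap stores the character, enables interaction and toggles a notification.
; InteractionObject waits, then a Translation timeline lerps the door's height, notifying the character and creating a completion message widget on every update.
; The construction script applies per-instance transforms to position door and generator independently.
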(event `self.Hitbox.OnComponentBeginOverlap`
  (params (OverlappedComponent :type "PrimitiveComponent Object Reference") (OtherActor :type "Actor Object Reference") (OtherComp :type "PrimitiveComponent Object Reference") (OtherBodyIndex :type Integer) (bFromSweep :type Boolean) (SweepResult :type "HitResult Structure (by ref)"))
  (bind _asbp_first_person_character (cast `/Game/FirstPersonBP/Blueprints/BP_FirstPersonCustom/BP_FirstPersonCharacter` OtherActor))
  (set `self.BP_FirstPerson` _asbp_first_person_character)
  (bind _output_get (set `self.CanInteract?` true))
  (`SceneComponent.SetVisibility` (`self.Notification`) _output_get false))

(event `self.Hitbox.OnComponentEndOverlap`
  (params (OverlappedComponent :type "PrimitiveComponent Object Reference") (OtherActor :type "Actor Object Reference") (OtherComp :type "PrimitiveComponent Object Reference") (OtherBodyIndex :type Integer))
  (cast `/Game/FirstPersonBP/Blueprints/BP_FirstPersonCustom/BP_FirstPersonCharacter` OtherActor)
  (bind _output_get (set `self.CanInteract?` false))
  (`SceneComponent.SetVisibility` (`self.Notification`) _output_get false))

(event `/Game/BP_Script/BP_Interface/BP_Interface_Interact.InteractionObject`
  (bind (_relativelocation_x _relativelocation_y _relativelocation_z) (`KismetMathLibrary.BreakVector` (`SceneComponent.RelativeLocation` (`self.Cube`))))
  (if (`self.CanInteract?`)
    (`KismetSystemLibrary.Delay` 3.0)
    (bind (_direction _newtrack_0) (`Timeline|Translation`)
      (:`Update`
        (bind (_returnvalue_x _returnvalue_y _returnvalue_z) (`KismetMathLibrary.BreakVector` (`KismetMathLibrary.VLerp` (`KismetMathLibrary.MakeVector` 0.0 _relativelocation_y _relativelocation_z) (`KismetMathLibrary.MakeVector` 0.0 _relativelocation_y 300.0) _newtrack_0)))
        (`SceneComponent.K2_SetRelativeLocation` (`self.Cube`) (`KismetMathLibrary.MakeVector` 0.0 _returnvalue_y _returnvalue_z) false false)
        (`|ExecutionSequence`
          (:`then_0`
            (message `/Game/BP_Script/BP_Interface/BP_Interface_Interact.NotificationEcranInteraction` (`self.BP_FirstPerson`) true))
          (:`then_1`
            (bind _returnvalue (`|CreateWidget` "/Game/BP_Script/BP_Widget/BP_Widget_MessageInteractionFinalisation.BP_Widget_MessageInteractionFinalisation_C" (`GameplayStatics.GetPlayerController` 0)))
            (`UserWidget.AddToViewport` _returnvalue 0)))))))

(fn `Porte`)

(fn `UserConstructionScript`
  (locals (NewLocalVar_0 :type "Vector Structure"))
  (bind _cube (`self.Cube`))
  (`|ExecutionSequence`
    (:`then_0`
      ;[1 1 1] Possibilité de pouvoir déplacer indépendemment
      (`SceneComponent.K2_SetRelativeLocationAndRotation` _cube (`self.TransformPorte`) (`self.RotatorPorte`) false false)
      (`SceneComponent.SetRelativeScale3D` _cube (`self.ScalePorte`)))
    (:`then_1`
      ;[1 1 1] Transform de l'enplacement de la génératrice
      (`SceneComponent.K2_SetRelativeLocationAndRotation` (`self.StaticMesh`) (`self.TransformGenerateur`) (`self.RotatorGenerateur`) false false)
      (`SceneComponent.SetRelativeScale3D` (`self.Cube`) (`self.ScalePorte`)))))