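; BP_DoorGenerateur is a double door, apparently tied to the generator objects, that swings open once.
; Its Porte event passes through a DoOnce that is never reset here, waits briefly, then plays the RotationPorte timeline.
; Separate timeline tracks blend the Droit and Gauche leaves' yaw toward their target rotations, lerping from the current yaw each update.
; Nothing in this graph triggers Porte or closes the door.
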(event `/Game/BP_Script/BP_Interface/BP_Interface_Interact.Porte`
  (bind _gauche (`self.Gauche`))
  (bind (_relativerotation_roll _relativerotation_pitch _relativerotation_yaw) (`KismetMathLibrary.BreakRotator` (`SceneComponent.RelativeRotation` (`self.Droit`))))
  (bind (_relativerotation_roll_2 _relativerotation_pitch_2 _relativerotation_yaw_2) (`KismetMathLibrary.BreakRotator` (`SceneComponent.RelativeRotation` _gauche)))
  (`/Engine/EditorBlueprintResources/StandardMacros.DoOnce` false
    (:`Completed`
      (`KismetSystemLibrary.Delay` 0.4)
      (bind (_direction _newtrack_0 _newtrack_1) (`Timeline|RotationPorte`)
        (:`Update`
          (`|ExecutionSequence`
            (:`then_0`
              ;[1 1 1] Animation de la porte droite qui s'ouvre
              (`SceneComponent.K2_SetRelativeRotation` (`self.Droit`) (`KismetMathLibrary.MakeRotator` 0.0 0.0 (`KismetMathLibrary.Lerp` _relativerotation_yaw (`self.RotationDroite`) _newtrack_0)) false false))
            (:`then_1`
              ;[1 1 1] Animation de la porte gauche
              (`SceneComponent.K2_SetRelativeRotation` _gauche (`KismetMathLibrary.MakeRotator` 0.0 0.0 (`KismetMathLibrary.Lerp` _relativerotation_yaw_2 (`self.RotationGauche`) _newtrack_1)) false false))))
        (:`Finished`
          (`KismetSystemLibrary.Delay` 0.4))))))

(fn `UserConstructionScript`)