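; Checkpoint actor that saves a new respawn point when the player character overlaps its trigger.
; On overlap it prints "Save" and writes SpawnLocation to BP_FirstPersonGameMode, converting the location from actor-local to world space.
; The saved rotation is copied untransformed and scale is reset to one.
; The construction script places CapsuleSpawn from separate LocationCapsule and RotationZ variables.
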(event `self.CollisionComponent.OnComponentBeginOverlap`
  (params (OverlappedComponent :type "PrimitiveComponent Object Reference") (OtherActor :type "Actor Object Reference") (OtherComp :type "PrimitiveComponent Object Reference") (OtherBodyIndex :type Integer) (bFromSweep :type Boolean) (SweepResult :type "HitResult Structure (by ref)"))
  (bind _spawn_location (`self.Spawn Location`))
  ;[1 1 1] Permet que lorsque le joueur touche la Triggerbox, sauvegarde la nouvelle location d'apparition
  (if (== OtherActor (`GameplayStatics.GetPlayerCharacter` 0))
    (`KismetSystemLibrary.PrintString` "Save")
    (bind _asbp_first_person_game_mode (cast `/Game/FirstPersonBP/Blueprints/BP_FirstPersonCustom/BP_FirstPersonGameMode` (`GameplayStatics.GetGameMode`)))
    (set `/Game/FirstPersonBP/Blueprints/BP_FirstPersonCustom/BP_FirstPersonGameMode.SpawnLocation` (`KismetMathLibrary.MakeTransform` (`KismetMathLibrary.TransformLocation` (`self.GetTransform`) (`KismetMathLibrary.MakeVector` (.x (.location _spawn_location)) (.y (.location _spawn_location)) (.z (.location _spawn_location)))) (.rotation _spawn_location)) _asbp_first_person_game_mode)))

(fn `UserConstructionScript`
  (`SceneComponent.K2_SetRelativeTransform` (`self.CapsuleSpawn`) (`KismetMathLibrary.MakeTransform` (`self.LocationCapsule`) (`KismetMathLibrary.MakeRotator` 0.0 0.0 (`self.Rotation Z`))) false false))